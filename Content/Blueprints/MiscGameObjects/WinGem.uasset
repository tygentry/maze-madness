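; WinGem is a gem actor that spins and floats up and down, with no overlap or win logic in its graphs.
; Each Tick adds local yaw at YawPerSecond, scaled by delta time.
; The bob adds a local Z offset of the sine of accumulated RunningTime times HeightScale every frame.
; That offset is not scaled by delta time, so bob height depends on frame rate.
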(event `self.ReceiveTick`
  (params (DeltaSeconds :type "Float (single-precision)"))
  ;[1 1 1] Rotation
  (`self.K2_AddActorLocalRotation` (`KismetMathLibrary.MakeRotator` 0.0 0.0 (* DeltaSeconds (`self.Yaw Per Second`))))
  ;[1 1 1] Float Up and Down
  (bind _output_get (set `self.Running Time` (+ DeltaSeconds (stale _output_get))))
  (`self.K2_AddActorLocalOffset` (`KismetMathLibrary.MakeVector` 0.0 0.0 (* (`KismetMathLibrary.Sin` _output_get) (`self.Height Scale`)))))

(fn `UserConstructionScript`)