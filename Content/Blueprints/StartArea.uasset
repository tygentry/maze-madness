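; Start area of the maze game, where the player places three keys to spawn the win gem.
; Each placement trigger shows a prompt widget if its key is held; E spawns that key at its spot, with input enabled only inside the InputSwap volume.
; Tick turns text toward the camera on yaw only and, once all keys are placed, spawns the gem, cuts the intense music and plays the end sound.
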(event `self.ReceiveBeginPlay`
  ;[1 1 1] Text Rotation and Continuous checking for End of Game
  (bind _returnvalue (`|CreateWidget` "/Game/UI/PlaceText.PlaceText_C" (`GameplayStatics.GetPlayerController` 0)))
  (set `self.PlaceText` _returnvalue))

(event `self.ReceiveTick`
  (params (DeltaSeconds :type "Float (single-precision)"))
  ;[1 1 1] Text Rotation and Continuous checking for End of Game
  (`self.GetAngle` null)
  (`self.GetAngle` null)
  (`self.GetAngle` null)
  (if (and (`self.PlacedKey1`) (`self.PlacedKey2`) (`self.PlacedKey3`))
    (if (not (`self.HasWon`))
      (`|SpawnActorFromClass` "/Game/Blueprints/WinGem.WinGem_C" (`SceneComponent.K2_GetComponentToWorld` (`self.SpawnWin`)) "Undefined" "OverrideRootScale" null null)
      (set `self.HasWon` true)
      (bind _asmaze_runner (cast `/Game/Blueprints/MazeRunner` (`GameplayStatics.GetPlayerCharacter` 0)))
      (`AudioComponent.FadeOut` (`/Game/Blueprints/MazeRunner.IntenseMusic` _asmaze_runner) 0.0 0.0)
      (`GameplayStatics.PlaySound2D` "/Game/Audio/GameEndSound_Cue.GameEndSound_Cue" 1.0 1.0 0.0 null null))))

(event `self.InputSwap.OnComponentBeginOverlap`
  (params (OverlappedComponent :type "PrimitiveComponent Object Reference") (OtherActor :type "Actor Object Reference") (OtherComp :type "PrimitiveComponent Object Reference") (OtherBodyIndex :type Integer) (bFromSweep :type Boolean) (SweepResult :type "HitResult Structure (by ref)"))
  ;[1 1 1] Turning On and Off Local Input
  (`self.EnableInput` (`GameplayStatics.GetPlayerController` 0)))

(event `self.KeyPlace1.OnComponentBeginOverlap`
  (params (OverlappedComponent :type "PrimitiveComponent Object Reference") (OtherActor :type "Actor Object Reference") (OtherComp :type "PrimitiveComponent Object Reference") (OtherBodyIndex :type Integer) (bFromSweep :type Boolean) (SweepResult :type "HitResult Structure (by ref)"))
  ;[1 1 1] Printing PlaceText to the User
  (if (`self.HasKey1`)
    (set `self.Visible` true)
    (set `self.Key` 0)
    (`UserWidget.AddToViewport` (`self.PlaceText`) 0 :!label _label)))

(event `Key|E`
  (params (Key :type "Key Structure"))
  ;[1 1 1] Reacting to Pickup of Key
  (:`Pressed`
    (switch `int` (`self.Key`)
      (:`0`
        (if (`self.HasKey1`)
          (`|SpawnActorFromClass` "/Game/Blueprints/Keys/KeyAqua/KeyAqua_Blueprint.KeyAqua_Blueprint_C" (`SceneComponent.K2_GetComponentToWorld` (`self.Spawn1`)) "Undefined" "OverrideRootScale" null null)
          (set `self.HasKey1` false)
          (set `self.PlacedKey1` true)
          (`WidgetLayoutLibrary.RemoveAllWidgets` :!label _label_2)))
      (:`1`
        (if (`self.HasKey2`)
          (`|SpawnActorFromClass` "/Game/Blueprints/Keys/KeyAztec/Key_Aztec_Low_Blueprint.Key_Aztec_Low_Blueprint_C" (`SceneComponent.K2_GetComponentToWorld` (`self.Spawn2`)) "Undefined" "OverrideRootScale" null null)
          (set `self.HasKey2` false)
          (set `self.PlacedKey2` true)
          (goto _label_2)))
      (:`2`
        (if (`self.HasKey3`)
          (`|SpawnActorFromClass` "/Game/Blueprints/Keys/KeyMining/KeyMining_Blueprint.KeyMining_Blueprint_C" (`SceneComponent.K2_GetComponentToWorld` (`self.Spawn3`)) "Undefined" "OverrideRootScale" null null)
          (set `self.HasKey3` false)
          (set `self.PlacedKey3` true)
          (goto _label_2))))))

(event `self.InputSwap.OnComponentEndOverlap`
  (params (OverlappedComponent :type "PrimitiveComponent Object Reference") (OtherActor :type "Actor Object Reference") (OtherComp :type "PrimitiveComponent Object Reference") (OtherBodyIndex :type Integer))
  ;[1 1 1] Turning On and Off Local Input
  (`self.DisableInput` (`GameplayStatics.GetPlayerController` 0)))

(event `self.KeyPlace1.OnComponentEndOverlap`
  (params (OverlappedComponent :type "PrimitiveComponent Object Reference") (OtherActor :type "Actor Object Reference") (OtherComp :type "PrimitiveComponent Object Reference") (OtherBodyIndex :type Integer))
  ;[1 1 1] Printing PlaceText to the User
  (if (`self.Visible`)
    (set `self.Visible` false)
    (`WidgetLayoutLibrary.RemoveAllWidgets` :!label _label_3)))

(event `self.KeyPlace2.OnComponentBeginOverlap`
  (params (OverlappedComponent :type "PrimitiveComponent Object Reference") (OtherActor :type "Actor Object Reference") (OtherComp :type "PrimitiveComponent Object Reference") (OtherBodyIndex :type Integer) (bFromSweep :type Boolean) (SweepResult :type "HitResult Structure (by ref)"))
  ;[1 1 1] Printing PlaceText to the User
  (if (`self.HasKey2`)
    (set `self.Visible` true)
    (set `self.Key` 1)
    (goto _label)))

(event `self.KeyPlace2.OnComponentEndOverlap`
  (params (OverlappedComponent :type "PrimitiveComponent Object Reference") (OtherActor :type "Actor Object Reference") (OtherComp :type "PrimitiveComponent Object Reference") (OtherBodyIndex :type Integer))
  ;[1 1 1] Printing PlaceText to the User
  (if (`self.Visible`)
    (set `self.Visible` false)
    (goto _label_3)))

(event `self.KeyPlace3.OnComponentBeginOverlap`
  (params (OverlappedComponent :type "PrimitiveComponent Object Reference") (OtherActor :type "Actor Object Reference") (OtherComp :type "PrimitiveComponent Object Reference") (OtherBodyIndex :type Integer) (bFromSweep :type Boolean) (SweepResult :type "HitResult Structure (by ref)"))
  ;[1 1 1] Printing PlaceText to the User
  (if (`self.HasKey3`)
    (set `self.Visible` true)
    (set `self.Key` 2)
    (goto _label)))

(event `self.KeyPlace3.OnComponentEndOverlap`
  (params (OverlappedComponent :type "PrimitiveComponent Object Reference") (OtherActor :type "Actor Object Reference") (OtherComp :type "PrimitiveComponent Object Reference") (OtherBodyIndex :type Integer))
  ;[1 1 1] Printing PlaceText to the User
  (if (`self.Visible`)
    (set `self.Visible` false)
    (goto _label_3)))

(fn `GetAngle`
  (params (Text :type "TextRenderComponent Object Reference"))
  (`SceneComponent.K2_SetWorldRotation` Text (`KismetMathLibrary.Conv_VectorToRotator` (`KismetMathLibrary.Normal` (* (- (`PlayerCameraManager.GetCameraLocation` (`GameplayStatics.GetPlayerCameraManager` 0)) (`SceneComponent.K2_GetComponentLocation` Text)) (1.0 1.0 0.0)))) false false))

(fn `UserConstructionScript`)